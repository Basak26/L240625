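; Player-controlled P38 pawn, apparently an aircraft, that flies forward constantly, steers by pitch and roll, and fires rockets.
; Tick feeds the forward vector into movement input, scaled by a Booster value that is raised while the Booster action is held and halved on release.
; Pitch and roll axes apply frame-rate-independent local rotations, so flight follows the nose.
; Attack spawns a BP_Rocket at the Arrow component's transform.
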(event `self.ReceiveTick`
  (params (DeltaSeconds :type "Float (single-precision)"))
  ;[1 1 1] MoveForward
  (`self.AddMovementInput` (`self.GetActorForwardVector`) (`self.Booster`)))

(event `InputAxis|Pitch(UpDown)`
  (params (AxisValue :type "Float (single-precision)"))
  ;[1 1 1] MovePitch
  (`self.K2_AddActorLocalRotation` (`KismetMathLibrary.MakeRotator` 0.0 (* AxisValue 60.0 (`GameplayStatics.GetWorldDeltaSeconds`)))))

(event `InputAxis|Roll(LeftRight)`
  (params (AxisValue :type "Float (single-precision)"))
  ;[1 1 1] MoveRoll
  (`self.K2_AddActorLocalRotation` (`KismetMathLibrary.MakeRotator` (* AxisValue 60.0 (`GameplayStatics.GetWorldDeltaSeconds`)))))

(event `InputAction|Booster`
  (params (Key :type "Key Structure"))
  (:`Pressed`
    ;[1 1 1] Booster
    (set `self.Booster` 1.0))
  (:`Released`
    (set `self.Booster` 0.5)))

(event `InputAction|Attack`
  (params (Key :type "Key Structure"))
  (:`Pressed`
    ;[1 1 1] Attack
    (`|SpawnActorFromClass` "/Game/My/BP/BP_Rocket.BP_Rocket_C" (`SceneComponent.K2_GetComponentToWorld` (`self.Arrow`)) "Undefined" "MultiplyWithRoot" null null)))

(fn `UserConstructionScript`)